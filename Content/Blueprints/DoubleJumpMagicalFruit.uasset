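; Magical fruit pickup that grants the ThirdPersonCharacter a timed double jump and respawns after being collected.
; On overlap while visible, it sets the character's DoubleJumpTimer to Duration, starts the respawn countdown, and hides itself with collision disabled.
; Tick, throttled by a one-second Delay, decrements TimeUntilRespawn and restores visibility and collision once it reaches zero or below.
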(event `self.ReceiveActorBeginOverlap`
  (params (OtherActor :type "Actor Object Reference"))
  ;[1 0.6913 0.5907] Fruit Collection
  (if (`SceneComponent.IsVisible` (`self.StaticMeshComponent`))
    (bind _asthird_person_character (cast `/Game/ThirdPersonBP/Blueprints/ThirdPersonCharacter` OtherActor))
    (set `/Game/ThirdPersonBP/Blueprints/ThirdPersonCharacter.DoubleJumpTimer` (`self.Duration`) _asthird_person_character)
    (set `self.TimeUntilRespawn` (`self.RespawnTime`))
    (`SceneComponent.SetVisibility` (`self.StaticMeshComponent`) false true)
    (`PrimitiveComponent.SetCollisionEnabled` (`self.Capsule`) "NoCollision")
    (`PrimitiveComponent.SetCollisionEnabled` (`self.StaticMeshComponent`) "NoCollision")))

(event `self.ReceiveTick`
  (params (DeltaSeconds :type "Float (single-precision)"))
  ;[1 0.8045 0.5289] Respawn Timer
  (`KismetSystemLibrary.Delay` 1.0)
  (set `self.TimeUntilRespawn` (- (`self.TimeUntilRespawn`) 1))
  (if (<= (`self.TimeUntilRespawn`) 0)
    (`SceneComponent.SetVisibility` (`self.StaticMeshComponent`) true true)
    (`PrimitiveComponent.SetCollisionEnabled` (`self.Capsule`) "QueryAndPhysics")
    (`PrimitiveComponent.SetCollisionEnabled` (`self.StaticMeshComponent`) "QueryAndPhysics")))

(fn `UserConstructionScript`)